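; Player component that punishes falls beyond an allowed height with a scream, flailing montage, input lockout and ragdoll.
; Tick tracks the drop from the fall's start; landing triggers impact and pain sounds plus a pelvis-down ragdoll, held for a delay scaled by fall height.
; While ragdolling, a pelvis ground trace drags the capsule along with the body.
; Prototype state: debug prints, empty jump/sprint stubs, uncalled speed recovery and unreached scream cleanup.
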(event `self.ReceiveBeginPlay`
  (bind _returnvalue (`GameplayStatics.GetPlayerCharacter` 0))
  ;[0.2292 0.2292 0.2292] Delay Fall Monitoring at the beginning of game
  (`KismetSystemLibrary.Delay` 1.0)
  (set `self.CharacterMovement` (`Character.CharacterMovement` _returnvalue))
  (set `self.Mesh` (`Character.Mesh` _returnvalue))
  (set `self.Capsule Component` (`Character.CapsuleComponent` _returnvalue))
  (`self.InitialPhysics`)
  (set `self.ShouldMonitorFall?` true))

(event `self.ReceiveTick`
  (params (DeltaSeconds :type "Float (single-precision)"))
  (bind _painsounds (`self.PainSounds`))
  (bind _returnvalue (- (`self.StartZ`) (`.Z` (`KismetMathLibrary.BreakVector3f` (`Actor.K2_GetActorLocation` (`GameplayStatics.GetPlayerCharacter` 0))))))
  ;[0.2292 0.2292 0.2292] Check if player is falling
  (`self.UpdateCapsulePosition`)
  (`KismetSystemLibrary.Delay` 0.1)
  (if (`self.ShouldMonitorFall?`)
    (if (`NavMovementComponent.IsFalling` (`self.CharacterMovement`))
      ;[0.2292 0.2292 0.2292] Get Z Height at the begining of fall
      (`KismetSystemLibrary.PrintString` "Is Falling")
      (if (== (`self.StartZ`) 0.0)
        (bind _output_get (set `self.StartZ` (`.Z` (`KismetMathLibrary.BreakVector3f` (`Actor.K2_GetActorLocation` (`GameplayStatics.GetPlayerCharacter` 0))))))
        (`KismetSystemLibrary.PrintString` (`KismetStringLibrary.Concat_StrStr` (`KismetStringLibrary.Conv_DoubleToString` _output_get) "StartZ") true true (struct :`R` 0.116764 :`G` 1.0 :`B` 0.283611 :`A` 1.0) 10.0)
        (set `self.HasFallen` true)
        (else
          ;[0.2292 0.2292 0.2292] If Max Allowed Fall Height is reached Scream and Fall Animation
          (`KismetSystemLibrary.PrintString` (`KismetStringLibrary.Concat_StrStr` (`KismetStringLibrary.Conv_DoubleToString` (`KismetMathLibrary.Abs` _returnvalue)) "FirstFallHeight"))
          (if (>= _returnvalue (`self.AllowedFallHeight`))
            (if (not (`self.IsScreaming?`))
              ;;[1 1 1] Fall Scream
              (bind _returnvalue_2 (`GameplayStatics.SpawnSoundAttached` "/Game/SoundFX/FallPunishment/MSS_Scream.MSS_Scream" (`self.Mesh`) "None" (0.0 0.0 0.0) (struct) "KeepRelativeOffset" true 1.0 1.0 0.0 "/Game/SoundFX/SoundAttenuation/SA_Short.SA_Short" null))
              (set `self.ScreamSounds` _returnvalue_2)
              (set `self.IsScreaming?` true)
              (`|PlayMontage` (`self.Mesh`) "/Game/MImports/Mixamo/AM_Flailing.AM_Flailing"
                (:`then`
                  (`Actor.DisableInput` (`GameplayStatics.GetPlayerController` 0) null)))))))
      (elif (`self.HasFallen`)
        ;[0.2292 0.2292 0.2292] If Player has stopped falling check if Max Allowed Fall Height is Reached
        (if (!= (`self.StartZ`) 0.0)
          (if (>= (`KismetMathLibrary.Abs` (- (`self.StartZ`) (`.Z` (`KismetMathLibrary.BreakVector3f` (`Actor.K2_GetActorLocation` (`GameplayStatics.GetPlayerCharacter` 0)))))) (`self.AllowedFallHeight`))
            (`/Engine/EditorBlueprintResources/StandardMacros.DoOnce` false :!label _label
              (:`Completed`
                (`self.RagdollAnim`)
                ;[0.2292 0.2292 0.2292] Delay reenabling input for a duration based on Fall Height
                ;;[0.2292 0.2292 0.2292] Stop Scream, Thud & Pain Sounds
                (`GameplayStatics.SpawnSoundAttached` "/Game/SoundFX/HitSound/MSS_PlasticMeleeHit.MSS_PlasticMeleeHit" (`self.Mesh`) "None" (0.0 0.0 0.0) (struct) "KeepRelativeOffset" false 1.0 1.0 0.0 "/Game/SoundFX/SoundAttenuation/SA_Short.SA_Short" null)
                (set `self.IsScreaming?` false)
                (bind _returnvalue_3 (`GameplayStatics.SpawnSoundAttached` "/Game/SoundFX/FallPunishment/MSS_Pain.MSS_Pain" (`self.Mesh`) "None" (0.0 0.0 0.0) (struct) "KeepRelativeOffset" true 1.0 1.0 0.0 "/Game/SoundFX/SoundAttenuation/SA_Short.SA_Short" null))
                (set `self.PainSounds` _returnvalue_3)
                (bind _output_get_2 (set `self.FallHeight` (`KismetMathLibrary.Abs` (- (`self.StartZ`) (`.Z` (`KismetMathLibrary.BreakVector3f` (`Actor.K2_GetActorLocation` (`GameplayStatics.GetPlayerCharacter` 0))))))))
                (`KismetSystemLibrary.PrintString` (`KismetStringLibrary.Concat_StrStr` "FallHeight" (`KismetStringLibrary.Conv_DoubleToString` _output_get_2)) true true (struct :`R` 1.0 :`G` 0.836546 :`B` 0.111539 :`A` 1.0) 10.0)
                (bind _output_get_3 (set `self.FallDelayTime` (* (* (`self.FallHeight`) 0.001) (`self.FallHeightMultiplyer`))))
                (`KismetSystemLibrary.Delay` _output_get_3)
                (`self.RagdollEnd`)
                (`KismetSystemLibrary.Delay` 0.5)
                (`KismetSystemLibrary.PrintText` "Input Enabled")
                (`KismetSystemLibrary.PrintText` "END FALL FUNCTION" true true (struct :`R` 1.0 :`G` 0.05192 :`B` 0.048604 :`A` 1.0) 10.0)
                ;;[1 1 1] Stop Pain Sounds
                (`AudioComponent.Stop` _painsounds)
                (`self.K2_DestroyComponent` _painsounds)
                (`Actor.EnableInput` (`GameplayStatics.GetPlayerController` 0) null)
                (set `self.StartZ` 0.0)
                (set `self.FallHeight` 0.0)
                (set `self.HasFallen` false)
                (goto _label :!via `Reset`)))
            (else
              (set `self.StartZ` 0.0)
              (set `self.FallHeight` 0.0)
              (set `self.HasFallen` false))))))))

(event `InitialPhysics`
  ;[1 1 1] Initial Capsule Location
  (set `self.PelvisOffset` (`SceneComponent.RelativeLocation` (`self.Mesh`))))

(event `UpdateCapsulePosition`
  (bind _returnvalue (`SceneComponent.GetSocketLocation` (`self.Mesh`) "pelvis"))
  ;[1 1 1] Update Capsule Location During Ragdoll
  (if (`self.Ragdolling`)
    (bind (_outhit _returnvalue_2) (`KismetSystemLibrary.LineTraceSingle` :`Start` _returnvalue :`End` (+ _returnvalue (0.0 0.0 -100.0)) :`TraceChannel` "TraceTypeQuery1" :`DrawDebugType` "ForDuration"))
    (if _returnvalue_2
      (set `self.TargetGroundLocation` (`.Location` (`GameplayStatics.BreakHitResult` _outhit)))
      (else
        (set `self.TargetGroundLocation` (`SceneComponent.GetSocketLocation` (`self.Mesh`) "pelvis"))))
    (bind _output_get (set `self.MeshLocation` (- (`self.TargetGroundLocation`) (`self.PelvisOffset`))))
    (`SceneComponent.K2_SetWorldLocation` (`self.Capsule Component`) _output_get false false)))

(fn `DisableJump`
  ;[0.1354 0.1354 0.1354] Disable Jump in C++ via Cast
)

(fn `DisableSprint`
  ;[0.1979 0.1979 0.1979] Disable Sprint in C++ via Cast
)

(fn `DisblePlayerInput`
  (bind _ascharacter (cast `Character` (`self.GetOwner`)))
  (`Actor.DisableInput` _ascharacter null))

(fn `EnableJump`
  ;[0.2292 0.2292 0.2292] Enable Jump in C++ via Cast
)

(fn `EnablePlayerInput`
  (bind _ascharacter (cast `Character` (`self.GetOwner`)))
  (`Actor.EnableInput` _ascharacter null))

(fn `EnableSprint`
  ;[0.09896 0.09896 0.09896] Enable Sprint in C++ via Cast
)

(fn `RagdollAnim`
  (bind _mesh (`self.Mesh`))
  (if (`self.Ragdolling`)
    (`KismetSystemLibrary.PrintText` "AlreadyRagdolling")
    (else
      (`PrimitiveComponent.SetCollisionEnabled` _mesh "QueryAndPhysics")
      (`SkeletalMeshComponent.SetAllBodiesBelowSimulatePhysics` _mesh "pelvis" true true)
      (set `self.Ragdolling` true))))

(fn `RagdollEnd`
  (bind _mesh (`self.Mesh`))
  (`SkeletalMeshComponent.SetAllBodiesBelowSimulatePhysics` _mesh "pelvis" false true)
  (`PrimitiveComponent.SetCollisionEnabled` _mesh "NoCollision")
  (set `self.Ragdolling` false)
  (`KismetSystemLibrary.PrintText` "NotRagdolling"))

(fn `SlowRecovery`
  (params (FallDelayTime :type "Float (double-precision)"))
  (bind _charactermovement (`self.CharacterMovement`))
  (bind _charactermovement_2 (`self.CharacterMovement`))
  (bind _falldelaytime (`self.FallDelayTime`))
  (bind _charactermovement_3 (`self.CharacterMovement`))
  (bind _maxwalkspeed (`CharacterMovementComponent.MaxWalkSpeed` _charactermovement))
  (set `self.FallDelayTime` FallDelayTime)
  (`KismetSystemLibrary.PrintString` (`KismetStringLibrary.Concat_StrStr` (`KismetStringLibrary.Conv_DoubleToString` _falldelaytime) "Delay Time") true true (struct :`R` 1.0 :`G` 0.740248 :`B` 0.064166 :`A` 1.0) 10.0)
  (set `CharacterMovementComponent.MaxWalkSpeed` (+ (/ 600.0 _falldelaytime) (`CharacterMovementComponent.MaxWalkSpeed` _charactermovement_3)) _charactermovement_3)
  (set `CharacterMovementComponent.MaxWalkSpeedCrouched` (+ (`CharacterMovementComponent.MaxWalkSpeedCrouched` _charactermovement_3) (/ 200.0 _falldelaytime)) _charactermovement)
  (if (>= _maxwalkspeed 600.0)
    (set `CharacterMovementComponent.MaxWalkSpeed` 600.0 _charactermovement_2)
    (set `CharacterMovementComponent.MaxWalkSpeedCrouched` 200.0 _charactermovement_2)
    (`self.EnableSprint`)
    (`self.EnableJump`)
    (`KismetSystemLibrary.K2_ClearAndInvalidateTimerHandle` (`self.SpeedControlTimer`))
    (`KismetSystemLibrary.PrintString` "TimerCleared")
    (else
      (`KismetSystemLibrary.PrintString` (`KismetStringLibrary.Concat_StrStr` (`KismetStringLibrary.Conv_DoubleToString` _maxwalkspeed) "New Max Walk Speed") true true (struct :`R` 0.098552 :`G` 1.0 :`B` 0.663216 :`A` 1.0) 10.0))))