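; BP_SlowProjectile is a projectile that slows any BP_ToyboxCharacter it hits and expires after a ten-second lifespan.
; It binds to the ProjectileMovement stop event and reacts only when the hit actor casts to that character.
; On such a hit it plays a sound, calls SlowDown, stops moving and destroys its Sphere.
; The Projectile component then switches to physics-only simulation with gravity and a small upward impulse.
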(event `self.ReceiveBeginPlay`
  ;[1 1 1] Comment
  (add `ProjectileMovementComponent.OnProjectileStop` (`self.ProjectileMovement`) (delegate `OnProjectileStop_Event`))
  (`self.SetLifeSpan` 10.0))

(event `OnProjectileStop_Event`
  (params (ImpactResult :type "HitResult Structure (by ref)"))
  (bind _projectile (`self.Projectile`))
  (bind _asbp_toybox_character (cast `/Game/Characters/Shared/BP_ToyboxCharacter` ImpactResult_HitActor))
  (`GameplayStatics.PlaySoundAtLocation` null (`self.K2_GetActorLocation` _asbp_toybox_character) (struct) 1.0 1.0 0.0 "/Game/SoundFX/SoundAttenuation/SA_Short.SA_Short" null null null)
  (`/Game/Characters/Shared/BP_ToyboxCharacter.SlowDown` _asbp_toybox_character)
  (`MovementComponent.StopMovementImmediately` (`self.ProjectileMovement`))
  (`ActorComponent.K2_DestroyComponent` (`self.Sphere`))
  (`PrimitiveComponent.SetSimulatePhysics` _projectile true)
  (`PrimitiveComponent.SetEnableGravity` _projectile true)
  (`PrimitiveComponent.SetCollisionEnabled` _projectile "PhysicsOnly")
  (`PrimitiveComponent.AddImpulse` _projectile (0.0 0.0 10.0) "None" false))

(fn `UserConstructionScript`)