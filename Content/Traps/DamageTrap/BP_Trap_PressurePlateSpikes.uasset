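; Pressure plate spike trap that damages Toybox characters and triggers selected actors.
; Once active shortly after Begin Play, stepping on the box lowers the plate, plays a sound, calls Triggering and raises the spikes by timeline; leaving raises the plate and reverses the spikes.
; Spike overlap applies GE_Damage through the character's own Ability System Component, with random SetByCaller magnitude, then plays a hit sound.
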(event `self.ReceiveBeginPlay`
  ;[1 1 1] Begin Play -----> Setting the mechanism to ACTIVE
  (`parent.ReceiveBeginPlay`)
  (`KismetSystemLibrary.Delay` 0.2)
  (set `self.Active` true))

(event `self.Box.OnComponentBeginOverlap`
  (params (OverlappedComponent :type "PrimitiveComponent Object Reference") (OtherActor :type "Actor Object Reference") (OtherComp :type "PrimitiveComponent Object Reference") (OtherBodyIndex :type Integer) (bFromSweep :type Boolean) (SweepResult :type "HitResult Structure (by ref)"))
  ;[1 1 1] Standing on a plate
  ;[1 1 1] If the mechanism is active
  (if (`self.Active`)
    ;[1 1 1] Pressure the plate down
    (`SceneComponent.K2_SetRelativeLocation` (`self.ItemA`) (0.0 0.0 -10.0) false false)
    ;[1 1 1] Trigger all the selected actors
    (`self.Triggering` false)
    ;[1 1 1] Play a pressure sound effect
    (`GameplayStatics.PlaySoundAtLocation` (`self.PressureSound`) (`self.K2_GetActorLocation`) (struct) 1.0 1.0 0.0 null null null null)
    ;[1 1 1] Spikes popping out through a lerp (0.4s)
    (bind (_direction _alpha) (`Timeline|Spikes!` :!label _label)
      (:`Update`
        (`SceneComponent.K2_SetRelativeLocation` (`self.ItemB`) (`KismetMathLibrary.VLerp` (0.0 0.0 -37.0) (0.0 0.0 0.0) _alpha) false false)))))

(event `self.Box.OnComponentEndOverlap`
  (params (OverlappedComponent :type "PrimitiveComponent Object Reference") (OtherActor :type "Actor Object Reference") (OtherComp :type "PrimitiveComponent Object Reference") (OtherBodyIndex :type Integer))
  ;[1 1 1] Not standing on a plate
  ;[1 1 1] Bring the plate up
  (`SceneComponent.K2_SetRelativeLocation` (`self.ItemA`) (0.0 0.0 0.0) false false)
  (goto _label :!via `Reverse`))

(event `self.ItemB.OnComponentBeginOverlap`
  (params (OverlappedComponent :type "PrimitiveComponent Object Reference") (OtherActor :type "Actor Object Reference") (OtherComp :type "PrimitiveComponent Object Reference") (OtherBodyIndex :type Integer) (bFromSweep :type Boolean) (SweepResult :type "HitResult Structure (by ref)"))
  ;[1 1 1] Spikes dealing damage to anyone and anything that overlaps with them
  (bind _astoybox_character (cast `ToyboxCharacter` (`.HitActor` (`GameplayStatics.BreakHitResult` SweepResult))))
  (bind _returnvalue (`AbilitySystemBlueprintLibrary.GetAbilitySystemComponent` _astoybox_character))
  (bind _output_get (set `self.EffectContext` (`AbilitySystemComponent.MakeEffectContext` _returnvalue)))
  (bind _returnvalue_2 (`AbilitySystemBlueprintLibrary.AssignTagSetByCallerMagnitude` (`AbilitySystemComponent.MakeOutgoingSpec` _returnvalue "/Game/Core/SharedAbilities/GE_Damage.GE_Damage_C" 0.0 _output_get) (struct :`TagName` "MetaTag.Damage") (`KismetMathLibrary.RandomFloatInRange` 20.0 40.0)))
  (`AbilitySystemBlueprintLibrary.EffectContextAddHitResult` _output_get SweepResult true)
  (`KismetSystemLibrary.PrintString` (`KismetStringLibrary.Conv_BoolToString` (`AbilitySystemBlueprintLibrary.EffectContextHasHitResult` _output_get)))
  (`AbilitySystemComponent.BP_ApplyGameplayEffectSpecToSelf` _returnvalue _returnvalue_2)
  (`GameplayStatics.PlaySoundAtLocation` "/Game/Traps/DamageTurret/Sounds/MSS_DamageTurretHit.MSS_DamageTurretHit" (`SceneComponent.K2_GetComponentLocation` (`self.Box`)) (struct) 1.0 1.0 0.0 null null null null))

(fn `UserConstructionScript`
  (`parent.UserConstructionScript`))