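; Damage turret projectile that hurts a ToyboxCharacter it hits and then becomes a falling physics prop, with a ten-second lifespan.
; When projectile movement stops, it applies a GE_Damage spec to the character's ability system with set-by-caller magnitude and the hit result in context.
; After a character hit, it plays the impact sound, destroys its sphere and lets the mesh simulate physics with a small upward impulse.
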(event `self.ReceiveBeginPlay`
  ;[1 1 1] Comment
  (add `ProjectileMovementComponent.OnProjectileStop` (`self.ProjectileMovement`) (delegate `OnProjectileStop_Event`))
  (`self.SetLifeSpan` 10.0))

(event `OnProjectileStop_Event`
  (params (ImpactResult :type "HitResult Structure (by ref)"))
  (bind _projectile (`self.Projectile`))
  (bind _astoybox_character (cast `ToyboxCharacter` (`.HitActor` (`GameplayStatics.BreakHitResult` ImpactResult))))
  (bind _returnvalue (`AbilitySystemBlueprintLibrary.GetAbilitySystemComponent` _astoybox_character))
  (`/Engine/EditorBlueprintResources/StandardMacros.IsValid` _returnvalue
    (:`Is Valid`
      (bind _output_get (set `self.EffectContext` (`AbilitySystemComponent.MakeEffectContext` _returnvalue)))
      (bind _returnvalue_2 (`AbilitySystemBlueprintLibrary.AssignTagSetByCallerMagnitude` (`AbilitySystemComponent.MakeOutgoingSpec` _returnvalue "/Game/Core/SharedAbilities/GE_Damage.GE_Damage_C" 0.0 _output_get) (struct :`TagName` "MetaTag.Damage") 10.0))
      (`AbilitySystemBlueprintLibrary.EffectContextAddHitResult` _output_get ImpactResult true)
      (`AbilitySystemComponent.BP_ApplyGameplayEffectSpecToSelf` _returnvalue _returnvalue_2))
    (:`Is Not Valid`
      _))
  (`GameplayStatics.PlaySoundAtLocation` "/Game/Traps/DamageTurret/Sounds/MSS_DamageTurretHit.MSS_DamageTurretHit" (`SceneComponent.K2_GetComponentLocation` (`self.Projectile`)) (struct) 1.0 1.0 0.0 null null null null)
  (`MovementComponent.StopMovementImmediately` (`self.ProjectileMovement`))
  (`ActorComponent.K2_DestroyComponent` (`self.Sphere`))
  (`PrimitiveComponent.SetSimulatePhysics` _projectile true)
  (`PrimitiveComponent.SetEnableGravity` _projectile true)
  (`PrimitiveComponent.SetCollisionEnabled` _projectile "PhysicsOnly")
  (`PrimitiveComponent.AddImpulse` _projectile (0.0 0.0 10.0) "None" false))

(fn `UserConstructionScript`)