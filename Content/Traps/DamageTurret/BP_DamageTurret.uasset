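; Trap turret that turns toward the nearest sensed Team.Attacker character and fires damage projectiles in bursts.
; The FiringRange overlap tracks attackers in DetectedPlayers and runs a looping fire timer until the list empties.
; PawnSensing sightings drive rotation toward ClosestCharacter, chosen by FindClosestPlayer, whose MinDistance is never reset here.
; Each burst ends at MaxFireCount in a cooldown with reload sound, then re-evaluates the closest target.
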(event `self.PawnSensing.OnSeePawn`
  (params (Pawn :type "Pawn Object Reference"))
  (bind _asbp_toybox_character (cast `/Game/Characters/Shared/BP_ToyboxCharacter` Pawn))
  (bind _returnvalue (`ToyboxCharacter.GetToyboxAbilitySystemComponent` _asbp_toybox_character))
  (if (`KismetSystemLibrary.IsValid` _returnvalue)
    (if (`GameplayTagAssetInterface.HasMatchingGameplayTag` _returnvalue (struct :`TagName` "Team.Attacker"))
      (`/Engine/EditorBlueprintResources/StandardMacros.IsValid` (`self.ClosestCharacter`)
        (:`Is Valid`
          _)
        (:`Is Not Valid`
          (set `self.ClosestCharacter` _asbp_toybox_character)))
      (`self.FindClosestPlayer`)
      (`self.K2_SetActorRotation` (`KismetMathLibrary.FindLookAtRotation` (`self.K2_GetActorLocation`) (+ (`self.K2_GetActorLocation` (`self.ClosestCharacter`)) (0.0 0.0 -100.0)))))))

(event `self.FiringRange.OnComponentBeginOverlap`
  (params (OverlappedComponent :type "PrimitiveComponent Object Reference") (OtherActor :type "Actor Object Reference") (OtherComp :type "PrimitiveComponent Object Reference") (OtherBodyIndex :type Integer) (bFromSweep :type Boolean) (SweepResult :type "HitResult Structure (by ref)"))
  (bind _asbp_toybox_character (cast `/Game/Characters/Shared/BP_ToyboxCharacter` OtherActor))
  (bind _returnvalue (`ToyboxCharacter.GetToyboxAbilitySystemComponent` _asbp_toybox_character))
  (if (`KismetSystemLibrary.IsValid` _returnvalue)
    (if (`GameplayTagAssetInterface.HasMatchingGameplayTag` _returnvalue (struct :`TagName` "Team.Attacker"))
      (`KismetArrayLibrary.Array_AddUnique` (`self.DetectedPlayers`) _asbp_toybox_character)
      (set `self.FireCount` 0)
      (set `self.IsInCoolDown` false)
      (bind _returnvalue_2 (`KismetSystemLibrary.K2_SetTimerDelegate` (delegate `Fire Projectile`) 0.2 true))
      (set `self.FireEventTimer` _returnvalue_2)
      (`self.Fire Projectile`))))

(event `Fire Projectile`
  (if (not (`self.IsInCoolDown`))
    (set `self.FireCount` (+ (`self.FireCount`) 1))
    (`|SpawnActorFromClass` "/Game/Traps/DamageTurret/BP_DamageProjectile.BP_DamageProjectile_C" (`SceneComponent.K2_GetComponentToWorld` (`self.Arrow`)) "Undefined" "MultiplyWithRoot" null null)
    (`GameplayStatics.PlaySoundAtLocation` (`self.FireSound`) (`self.K2_GetActorLocation`) (struct) 1.0 1.0 0.0 (`self.Attenuation Settings`) null null null)
    (if (== (`self.FireCount`) (`self.MaxFireCount`))
      (`self.CoolDown`))))

(event `CoolDown`
  (set `self.IsInCoolDown` true)
  (bind _returnvalue (`GameplayStatics.SpawnSoundAtLocation` (`self.ReloadSound`) (`SceneComponent.K2_GetComponentLocation` (`self.Turret`)) (struct) 1.0 1.0 0.0 (`self.Attenuation Settings`) null))
  (`KismetSystemLibrary.Delay` (`self.CoolDownTime`))
  (`AudioComponent.Stop` _returnvalue)
  (`ActorComponent.K2_DestroyComponent` _returnvalue)
  (set `self.IsInCoolDown` false)
  (set `self.FireCount` 0)
  (`self.FindClosestPlayer`))

(event `self.FiringRange.OnComponentEndOverlap`
  (params (OverlappedComponent :type "PrimitiveComponent Object Reference") (OtherActor :type "Actor Object Reference") (OtherComp :type "PrimitiveComponent Object Reference") (OtherBodyIndex :type Integer))
  (bind _asbp_toybox_character (cast `/Game/Characters/Shared/BP_ToyboxCharacter` OtherActor))
  (bind _returnvalue (`KismetArrayLibrary.Array_RemoveItem` (`self.DetectedPlayers`) _asbp_toybox_character))
  (if _returnvalue
    (`self.FindClosestPlayer`)
    (if (== (`KismetArrayLibrary.Array_Length` (`self.DetectedPlayers`)) 0)
      (`KismetSystemLibrary.K2_ClearAndInvalidateTimerHandle` (`self.FireEventTimer`)))))

(fn `FindClosestPlayer`
  (bind _detectedplayers (`self.DetectedPlayers`))
  (if (!= (`KismetArrayLibrary.Array_Length` _detectedplayers) 0)
    (if (== (`KismetArrayLibrary.Array_Length` _detectedplayers) 1)
      (set `self.ClosestCharacter` (`|GetArrayItem` (`self.DetectedPlayers`)))
      (else
        (for _array_element _detectedplayers
          (bind _output_get (set `self.CurrentDistance` (`self.GetDistanceTo` _array_element)))
          (if (< _output_get (`self.MinDistance`))
            (set `self.MinDistance` (`self.CurrentDistance`))
            (set `self.ClosestCharacter` _array_element)))))))

(fn `UserConstructionScript`)