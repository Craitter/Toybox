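; Shield generator trap actor that counts hits on its Generator component and damages the defender's shield once the hit limit is reached.
; At the limit it searches all BP_ToyboxCharacter actors for the Team.Defender gameplay tag and applies GE_DamageShield to each match through its AbilitySystem.
; The generator destroys itself inside that loop, so only when a defender is found, and debug prints trace the process.
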(event `self.Generator.OnComponentHit`
  (params (HitComponent :type "PrimitiveComponent Object Reference") (OtherActor :type "Actor Object Reference") (OtherComp :type "PrimitiveComponent Object Reference") (NormalImpulse :type "Vector Structure") (Hit :type "HitResult Structure (by ref)"))
  (bind _output_get (set `self.HitCounter` (+ (`self.HitCounter`) 1)))
  (if (>= _output_get (`self.HitMax`))
    (`KismetSystemLibrary.PrintText` "MaxHIt")
    (bind _outactors (`GameplayStatics.GetAllActorsOfClass` "/Game/Characters/Shared/BP_ToyboxCharacter.BP_ToyboxCharacter_C"))
    (for _array_element _outactors
      (bind _returnvalue (`AbilitySystemBlueprintLibrary.GetAbilitySystemComponent` _array_element))
      (bind _returnvalue_2 (`GameplayTagAssetInterface.HasMatchingGameplayTag` _returnvalue (struct :`TagName` "Team.Defender")))
      (`KismetSystemLibrary.PrintString` (`KismetStringLibrary.Conv_BoolToString` _returnvalue_2))
      (if _returnvalue_2
        (bind _output_get_2 (set `self.Defender` _array_element))
        (`KismetSystemLibrary.PrintString` (`KismetSystemLibrary.GetDisplayName` _output_get_2) true true (struct :`G` 0.66 :`B` 1.0 :`A` 1.0) 20.0)
        (`AbilitySystemComponent.BP_ApplyGameplayEffectToTarget` :`self` (`self.AbilitySystem`) :`GameplayEffectClass` "/Game/Traps/Shield/GE_DamageShield.GE_DamageShield_C" :`Target` _returnvalue)
        (`self.K2_DestroyActor`)))))

(fn `UserConstructionScript`)