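; Destructible shield generator that applies GE_DamageShield to the match's defender when it dies.
; BeginPlay gives the Orb a dynamic aura material and caches MaxHealth from the actor's Health attribute set.
; Health changes drive the red channel of the Orb's Tint up as health drops.
; On death, its ability system applies the effect to the defender's ability system from MatchGameState, then destroys only the Orb component.
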(event `self.ReceiveBeginPlay`
  (bind _orb (`self.Orb`))
  (bind _returnvalue (`PrimitiveComponent.CreateDynamicMaterialInstance` _orb 0 "/Game/MImports/sA_Megapack_v1/sA_SkillSet_1/Materials/MI_Aura_2.MI_Aura_2" "None"))
  (`PrimitiveComponent.SetMaterial` _orb 0 _returnvalue)
  (bind _returnvalue_2 (`AbilitySystemComponent.GetAttributeSet` (`self.AbilitySystemComponent`) "/Script/Toybox.HealthAttributeSet"))
  (bind _ashealth_attribute_set (cast `HealthAttributeSet` _returnvalue_2))
  (bind (_maxhealth_basevalue _maxhealth_currentvalue) (break `GameplayAttributeData` (`HealthAttributeSet.MaxHealth` _ashealth_attribute_set)))
  (set `self.MaxHealth` _maxhealth_currentvalue))

(event `self.K2_OnDeath`
  (bind _asmatch_game_state (cast `MatchGameState` (`GameplayStatics.GetGameState`)))
  (`AbilitySystemComponent.BP_ApplyGameplayEffectToTarget` :`self` (`self.AbilitySystemComponent`) :`GameplayEffectClass` "/Game/Traps/Shield/GE_DamageShield.GE_DamageShield_C" :`Target` (`MatchGameState.GetDefenderAbilitySystemComponent` _asmatch_game_state))
  (`ActorComponent.K2_DestroyComponent` (`self.Orb`)))

(event `self.K2_OnHealthChanged`
  (params (NewHealth :type "Float (single-precision)"))
  (`MeshComponent.SetVectorParameterValueOnMaterials` (`self.Orb`) "Tint" (`KismetMathLibrary.MakeVector` (* (- 1.0 (/ NewHealth (`self.MaxHealth`))) 255.0))))

(fn `UserConstructionScript`)