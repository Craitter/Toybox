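; Ammo refill zone that gradually restores weapon ammo to a Toybox character standing inside its sphere.
; Entering adds replicated gameplay tags, caches the character's ability system and weapon attributes, and starts a one-second looping timer.
; Each tick applies GE_AmmoRefill with a SetByCaller magnitude of a rounded tenth of max ammo.
; Any end overlap stops the timer and removes the tags from the last cast character.
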(event `self.Sphere.OnComponentBeginOverlap`
  (params (OverlappedComponent :type "PrimitiveComponent Object Reference") (OtherActor :type "Actor Object Reference") (OtherComp :type "PrimitiveComponent Object Reference") (OtherBodyIndex :type Integer) (bFromSweep :type Boolean) (SweepResult :type "HitResult Structure (by ref)"))
  (bind _asbp_toybox_character (cast `/Game/Characters/Shared/BP_ToyboxCharacter` OtherActor))
  (`AbilitySystemBlueprintLibrary.AddLooseGameplayTags` _asbp_toybox_character (`self.Gameplay Tags`) true)
  (bind _output_get (set `self.OverlappingCharacter` _asbp_toybox_character))
  (bind _returnvalue (`AbilitySystemBlueprintLibrary.GetAbilitySystemComponent` _output_get))
  (set `self.AbilitySystemComponent` _returnvalue)
  (bind _returnvalue_2 (`AbilitySystemComponent.GetAttributeSet` _returnvalue "/Script/Toybox.WeaponAttributeSet"))
  (bind _asweapon_attribute_set (cast `WeaponAttributeSet` _returnvalue_2))
  (bind _output_get_2 (set `self.WeaponAttribute Set` _asweapon_attribute_set))
  (bind _currentammo (`WeaponAttributeSet.CurrentAmmo` _output_get_2))
  (set `self.Current Ammo` _currentammo)
  (set `self.MaxAmmo` (`.CurrentValue` (break `GameplayAttributeData` (`WeaponAttributeSet.MaxAmmo` _output_get_2))))
  (set `self.CurrentAmmo` (`.CurrentValue` (break `GameplayAttributeData` _currentammo)))
  (`KismetSystemLibrary.K2_SetTimer` null "IncrementAmmo" 1.0 true))

(event `self.Sphere.OnComponentEndOverlap`
  (params (OverlappedComponent :type "PrimitiveComponent Object Reference") (OtherActor :type "Actor Object Reference") (OtherComp :type "PrimitiveComponent Object Reference") (OtherBodyIndex :type Integer))
  (`KismetSystemLibrary.K2_ClearTimer` null "IncrementAmmo")
  (`AbilitySystemBlueprintLibrary.RemoveLooseGameplayTags` (stale `self.Sphere.OnComponentBeginOverlap` _asbp_toybox_character) (`self.Gameplay Tags`) true))

(fn `IncrementAmmo`
  (bind _abilitysystemcomponent (`self.AbilitySystemComponent`))
  (bind _output_get (set `self.IncrementValue` (`KismetMathLibrary.Conv_IntToDouble` (`KismetMathLibrary.Round` (* (`self.MaxAmmo`) 0.1)))))
  (bind _returnvalue (`AbilitySystemBlueprintLibrary.AssignTagSetByCallerMagnitude` (`AbilitySystemComponent.MakeOutgoingSpec` :`self` _abilitysystemcomponent :`GameplayEffectClass` "/Game/Traps/AmmoRefill/GE_AmmoRefill.GE_AmmoRefill_C") (struct :`TagName` "MetaTag.RefillAmmo") _output_get))
  (`AbilitySystemComponent.BP_ApplyGameplayEffectSpecToSelf` _abilitysystemcomponent _returnvalue)
  (set `self.CurrentAmmo` (+ (`self.CurrentAmmo`) (`self.IncrementValue`))))

(fn `UserConstructionScript`)