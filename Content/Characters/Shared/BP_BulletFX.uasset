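; BP_BulletFX is a shared component that plays a bullet's firing effects through a single TriggerFireFX function.
; It spawns a scaled muzzle flash, with auto-destroy off, and a fire sound at the owner's root location.
; A flight sound attaches to the owner's root and stops when that is destroyed.
; The auto-destroying trail effect attaches to that sound's audio component rather than directly to the root.
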(fn `Trigger Fire FX`
  (bind _attenuation_settings (`self.Attenuation Settings`))
  (bind _rootcomponent (`Actor.RootComponent` (`self.GetOwner`)))
  (bind _returnvalue (`SceneComponent.K2_GetComponentLocation` _rootcomponent))
  (`NiagaraFunctionLibrary.SpawnSystemAtLocation` (`self.MuzzleFlashFX`) _returnvalue (struct) (`self.MuzzleFlashFXScale`) false)
  (`GameplayStatics.PlaySoundAtLocation` (`self.FireSFX`) _returnvalue (struct) 1.0 1.0 0.0 _attenuation_settings null null null)
  (bind _returnvalue_2 (`GameplayStatics.SpawnSoundAttached` (`self.BulletFlightSFX`) _rootcomponent "None" (0.0 0.0 0.0) (struct) "KeepRelativeOffset" true 1.0 1.0 0.0 _attenuation_settings null))
  (`NiagaraFunctionLibrary.SpawnSystemAttached` (`self.BulletTrailFX`) _returnvalue_2 "None" (0.0 0.0 0.0) (struct) "KeepRelativeOffset" true))