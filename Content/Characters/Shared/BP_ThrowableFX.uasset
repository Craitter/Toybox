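; BP_ThrowableFX is a component that plays sound and particle effects for its owning throwable.
; Throwing attaches a timer sound to the owner's root, stopped when the owner is destroyed, and attaches the throw particle system to that audio component.
; Activation spawns a one-shot sound and scaled particle system at a given location.
; Bounces play a sound at the impact point, throttled by a game-time cooldown.
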(event `DeleteMe`)

(fn `Trigger Bounce FX`
  (params (BounceLocation :type "Vector Structure"))
  (bind _returnvalue (`KismetSystemLibrary.GetGameTimeInSeconds`))
  (if (<= (`self.BounceCooldown`) (- _returnvalue (`self.LastBounce`)))
    (set `self.LastBounce` _returnvalue)
    (`GameplayStatics.PlaySoundAtLocation` (`self.BounceSFX`) BounceLocation (struct) 1.0 1.0 0.0 (`self.BounceAttenuation`) null null null)))

(fn `Trigger Throw FX`
  (bind _returnvalue (`GameplayStatics.SpawnSoundAttached` (`self.ThrowTimerSFX`) (`Actor.RootComponent` (`self.GetOwner`)) "None" (0.0 0.0 0.0) (struct) "KeepRelativeOffset" true 1.0 1.0 0.0 "/Game/SoundFX/SoundAttenuation/SA_Short.SA_Short" null))
  (`NiagaraFunctionLibrary.SpawnSystemAttached` (`self.ThrowFX`) _returnvalue "None" (0.0 0.0 0.0) (struct) "KeepRelativeOffset" true))

(fn `Trigger Throwable Activation FX`
  (params (ThrowableLocation :type "Vector Structure"))
  (`GameplayStatics.SpawnSoundAtLocation` (`self.ThrowActivationSFX`) ThrowableLocation (struct) 1.0 1.0 0.0 (`self.ActivationAttenuation`) null)
  (bind _returnvalue (`NiagaraFunctionLibrary.SpawnSystemAtLocation` (`self.ThrowActivationFX`) ThrowableLocation (struct) (`self.ThrowActivationScale`) true false))
  (`self.Activate` _returnvalue false))