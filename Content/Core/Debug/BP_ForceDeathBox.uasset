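; Debug volume that deals lethal-scale damage to a Toybox character entering its box.
; On begin overlap it applies GE_Damage to the character's own ability system component, with a large fixed SetByCaller magnitude on MetaTag.Damage.
; It tracks one overlapping actor at a time, storing the effect handle and ability system to remove the effect when that actor leaves.
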(event `self.ReceiveTick`
  (params (DeltaSeconds :type "Float (single-precision)")))

(event `self.Box.OnComponentBeginOverlap`
  (params (OverlappedComponent :type "PrimitiveComponent Object Reference") (OtherActor :type "Actor Object Reference") (OtherComp :type "PrimitiveComponent Object Reference") (OtherBodyIndex :type Integer) (bFromSweep :type Boolean) (SweepResult :type "HitResult Structure (by ref)"))
  (if (`KismetSystemLibrary.IsValid` (`self.OverlappingActor`))
    _
    (elif (`KismetSystemLibrary.DoesImplementInterface` OtherActor "/Script/GameplayAbilities.AbilitySystemInterface")
      (bind _astoybox_character (cast `ToyboxCharacter` OtherActor))
      (bind _returnvalue (`ToyboxCharacter.GetToyboxAbilitySystemComponent` _astoybox_character))
      (if (`KismetSystemLibrary.IsValid` _returnvalue)
        (set `self.OverlappingActor` OtherActor)
        (bind _returnvalue_2 (`AbilitySystemBlueprintLibrary.AssignTagSetByCallerMagnitude` (`AbilitySystemComponent.MakeOutgoingSpec` _returnvalue "/Game/Core/SharedAbilities/GE_Damage.GE_Damage_C" 0.0 (`AbilitySystemComponent.MakeEffectContext` _returnvalue)) (struct :`TagName` "MetaTag.Damage") 1000.0))
        (bind _returnvalue_3 (`AbilitySystemComponent.BP_ApplyGameplayEffectSpecToSelf` _returnvalue _returnvalue_2))
        (set `self.EffectSpec` _returnvalue_3)
        (set `self.abilitySystem` _returnvalue)))))

(event `self.Box.OnComponentEndOverlap`
  (params (OverlappedComponent :type "PrimitiveComponent Object Reference") (OtherActor :type "Actor Object Reference") (OtherComp :type "PrimitiveComponent Object Reference") (OtherBodyIndex :type Integer))
  (if (== OtherActor (`self.OverlappingActor`))
    (`AbilitySystemComponent.RemoveActiveGameplayEffect` (`self.abilitySystem`) (`self.EffectSpec`) -1)
    (set `self.OverlappingActor` null)))

(fn `UserConstructionScript`)